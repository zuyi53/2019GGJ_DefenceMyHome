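; BP_targetpoint is a monster spawner that creates Monster1 AI pawns at its own location.
; It spawns one on BeginPlay, then uses a 10-second Delay on Tick as a repeating timer.
; Each cycle decrements MaxSpawn and spawns again only while the count stays above zero and GS_LEVEL1's PlayerWin flag is false.
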(event EventBeginPlay
  (AI|SpawnAIFromClass "/Game/Blueprints/monster1.monster1_C" 0 (Transformation|GetActorLocation) "0, 0, 0" false))

(event EventTick
  (params (DeltaSeconds :type Float%20%28single-precision%29))
  (bind _max_spawn (Variables|Default|Getmax%20spawn))
  (Utilities|FlowControl|Delay 1e+01)
  (Math|Integer|DecrementInt _max_spawn
    (:%20%20
      (if (> _max_spawn 0)
        (if (not (Variables|/Game/Blueprints/GS_LEVEL1.GS_LEVEL1_C|Getplayer%20win (.AsGS%20LEVEL1 (Utilities|Casting|CastToGS_LEVEL1 (Game|GetGameState)))))
          (AI|SpawnAIFromClass "/Game/Blueprints/monster1.monster1_C" 0 (Transformation|GetActorLocation) "0, 0, 0" false))))))

(fn ConstructionScript)
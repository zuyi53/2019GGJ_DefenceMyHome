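; Trigger actor that shows a dialog widget when the player overlaps it, chosen by the FirstPersonCharacter's GotWeapon flag.
; A DoOnce gates the overlap, then Dialog1 (has weapon) or Dialog2 (no weapon) opens with UI-focused input and a visible cursor.
; End overlap by any actor removes only the stored Dialog2, restores game-only input, hides the cursor and resets the gate.
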(event EventBeginPlay)

(event Collision|EventActorBeginOverlap
  (params (OtherActor :type Actor%20Object%20Reference))
  (bind _returnvalue (Game|GetPlayerController 0))
  (bind _returnvalue_2 (Game|GetPlayerController 0))
  (if (== OtherActor (Game|GetPlayerCharacter 0))
    (Utilities|FlowControl|DoOnce false
      (:Completed
        (if (Variables|/Game/Blueprints/FirstPersonCharacter.FirstPersonCharacter_C|Getgot%20weapon? (.AsFirst%20Person%20Character (Utilities|Casting|CastToFirstPersonCharacter (Game|GetPlayerCharacter 0))))
          (bind _returnvalue_3 (UserInterface|CreateWidget "/Game/widget/dialog1.dialog1_C"))
          (UserInterface|Viewport|AddtoViewport _returnvalue_3 0)
          (Input|SetInputModeGameandUI _returnvalue _returnvalue_3 "DoNotLock" true)
          (Variables|/Script/Engine.PlayerController|SetbShowMouseCursor _returnvalue true)
          (else
            (bind _returnvalue_4 (UserInterface|CreateWidget "/Game/widget/dialog2.dialog2_C"))
            (Variables|Default|Setdialog2 _returnvalue_4)
            (UserInterface|Viewport|AddtoViewport _returnvalue_4 0)
            (Input|SetInputModeGameandUI _returnvalue_2 _returnvalue_4 "DoNotLock" true)
            (Variables|/Script/Engine.PlayerController|SetbShowMouseCursor _returnvalue_2 true)))))))

(event EventTick
  (params (DeltaSeconds :type Float%20%28single-precision%29)))

(event Collision|EventActorEndOverlap
  (params (OtherActor :type Actor%20Object%20Reference))
  (bind _returnvalue (Game|GetPlayerController 0))
  (bind _returnvalue_2 (Game|GetPlayerController 0))
  (bind _returnvalue_3 (Game|GetPlayerController 0))
  (Widget|RemovefromParent (Variables|Default|Getdialog2))
  (Input|SetInputModeGameOnly _returnvalue)
  (Variables|/Script/Engine.PlayerController|SetbShowMouseCursor _returnvalue false)
  (Utilities|FlowControl|DoOnce false) ; enters at Reset
)

(fn ConstructionScript)
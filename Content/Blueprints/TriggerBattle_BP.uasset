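; Trigger actor that shows a Dialog1 widget when the player character overlaps it, presumably as a lead-in to a battle.
; A DoOnce gates widget creation, then switches to game-and-UI input focused on the dialog with the mouse cursor shown.
; End overlap, which does not check the overlapping actor, removes the dialog, restores game-only input, hides the cursor and resets the DoOnce.
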(event EventBeginPlay)

(event Collision|EventActorBeginOverlap
  (params (OtherActor :type Actor%20Object%20Reference))
  (bind _returnvalue (Game|GetPlayerController 0))
  (if (== OtherActor (Game|GetPlayerCharacter 0))
    (Utilities|FlowControl|DoOnce false
      (:Completed
        (bind _returnvalue_2 (UserInterface|CreateWidget "/Game/widget/dialog1.dialog1_C"))
        (Variables|Default|Setdialog1 _returnvalue_2)
        (UserInterface|Viewport|AddtoViewport _returnvalue_2 0)
        (Input|SetInputModeGameandUI _returnvalue _returnvalue_2 "DoNotLock" true)
        (Variables|/Script/Engine.PlayerController|SetbShowMouseCursor _returnvalue true)))))

(event EventTick
  (params (DeltaSeconds :type Float%20%28single-precision%29)))

(event Collision|EventActorEndOverlap
  (params (OtherActor :type Actor%20Object%20Reference))
  (bind _returnvalue (Game|GetPlayerController 0))
  (bind _returnvalue_2 (Game|GetPlayerController 0))
  (Widget|RemovefromParent (Variables|Default|Getdialog1))
  (Input|SetInputModeGameOnly _returnvalue)
  (Variables|/Script/Engine.PlayerController|SetbShowMouseCursor _returnvalue false)
  (Utilities|FlowControl|DoOnce false) ; enters at Reset
)

(fn ConstructionScript)
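; BP_GUN is an actor that removes itself once the player's FirstPersonCharacter shows its FPGun, apparently a pickup or world gun.
; BeginPlay caches the player character.
; Tick polls through a 0.2-second Delay and destroys the actor when the FPGun component is visible, with no overlap logic of its own.
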(event EventBeginPlay
  (bind _asfirst_person_character (Utilities|Casting|CastToFirstPersonCharacter (Game|GetPlayerCharacter 0)))
  (Variables|Default|Setplayer _asfirst_person_character))

(event Collision|EventActorBeginOverlap
  (params (OtherActor :type Actor%20Object%20Reference)))

(event EventTick
  (params (DeltaSeconds :type Float%20%28single-precision%29))
  (bind _player (Variables|Default|Getplayer))
  (Utilities|FlowControl|Delay 0.2)
  (Utilities|IsValid _player
    (:Is%20Valid
      (if (Variables|/Script/Engine.SceneComponent|GetbVisible (Variables|/Game/Blueprints/FirstPersonCharacter.FirstPersonCharacter_C|GetFP_Gun _player))
        (Actor|DestroyActor)))))

(fn ConstructionScript)
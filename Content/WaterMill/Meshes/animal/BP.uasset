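; Animal actor from the WaterMill content that moves a dove along a spline path in a continuous loop.
; BeginPlay offsets the dove's animation by AnimPos, caches the spline length and starts at the spline's far end.
; A 0.01-second looping timer, rather than Tick, steps the distance backward by Speed, applies the spline's location and rotation with sweep, and wraps around at zero.
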(event Custom|Kre
  (Utilities|FlowControl|Sequence
    (:then_0
      (Variables|Default|Setpos (- (Variables|Default|Getpos) (Math|Conversions|ToFloat(Integer) (Variables|Default|GetSpeed))))
      (Transformation|SetWorldLocationAndRotation (Spline|GetLocationatDistanceAlongSpline (Variables|Default|GetSpline) (stale EventBeginPlay _output_get_2) "World") (stale _output_get) true false :!label _label))
    (:then_1
      (bind _output_get (Variables|Default|Setrot (Spline|GetRotationatDistanceAlongSpline (Variables|Default|GetSpline) (Variables|Default|Getpos) "World")))
      (goto _label))
    (:then_2
      (if (<= (Variables|Default|Getpos) 0.0)
        (Variables|Default|Setpos (+ (Variables|Default|Getpos) (stale EventBeginPlay _output_get)))
        (goto _label)))))

(event EventBeginPlay
  (Components|Animation|SetPosition (Variables|Default|GetDove) (Variables|Default|GetAnimPos) true)
  (Utilities|Time|SetTimerbyFunctionName 0 "Kre" 0.01 true)
  (bind _output_get (Variables|Default|SetDist (Spline|GetSplineLength)))
  (bind _output_get_2 (Variables|Default|Setpos _output_get))
  (Transformation|SetWorldLocationAndRotation (Spline|GetLocationatDistanceAlongSpline (Variables|Default|GetSpline) _output_get_2 "World") (stale Custom|Kre _output_get) true false))

(event Collision|EventActorBeginOverlap
  (params (OtherActor :type Actor%20Object%20Reference)))

(event EventTick
  (params (DeltaSeconds :type Float%20%28single-precision%29)))

(fn ConstructionScript)